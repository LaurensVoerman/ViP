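; VR push button that resets, saves or loads the lab scene's pickup items, depending on its Function setting.
; Overlapping motion controllers drive button travel along its up vector, firing at maximum travel.
; Save passes all pickups to MySaveGame; Load, also run at BeginPlay, and Reset share one rebuild path that spawns or finds items and reconnects tubes.
; Reset starts from an empty save containing only the shutter (schuifraam), which Load adds if missing.
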(event `self.VRButton.OnComponentBeginOverlap`
  (params (OverlappedComponent :type "PrimitiveComponent Object Reference") (OtherActor :type "Actor Object Reference") (OtherComp :type "PrimitiveComponent Object Reference") (OtherBodyIndex :type Integer) (bFromSweep :type Boolean) (SweepResult :type "HitResult Structure (by ref)"))
  (bind _asbp_motion_controller (cast `/Game/VirtualRealityBP/Blueprints/BP_MotionController` OtherActor))
  (bind _output_get (set `self.Tracking MC` (`/Game/VirtualRealityBP/Blueprints/BP_MotionController.MotionController` _asbp_motion_controller)))
  (set `self.MC Initial Location` (`SceneComponent.K2_GetComponentLocation` _output_get))
  (set `self.Is Tracking` true))

(event `self.ReceiveTick`
  (params (DeltaSeconds :type "Float (single-precision)"))
  (if (`self.Is Tracking`)
    (set `self.Current Travel` (`KismetMathLibrary.FClamp` (`KismetMathLibrary.Abs` (`KismetMathLibrary.VSize` (`KismetMathLibrary.ProjectVectorOnToVector` (- (`SceneComponent.K2_GetComponentLocation` (`self.Tracking MC`)) (`self.MC Initial Location`)) (`SceneComponent.GetUpVector` (`self.VRButton`))))) 0.0 (`self.Maximum Travel`)))
    (bind _output_get (set `self.Button Current Location` (- (`self.Button Initial Location`) (* (`SceneComponent.GetUpVector` (`self.VRButton`)) (`self.Current Travel`)))))
    (`SceneComponent.K2_SetWorldLocation` (`self.VRButton`) _output_get false false)
    (if (>= (`self.Current Travel`) (`self.Maximum Travel`))
      (`self.Fully Pressed`))))

(event `Fully Pressed`
  (bind _returnvalue (`KismetMathLibrary.MakeTransform` (0.0 0.0 0.0)))
  (bind _newpickupcubes (`self.NewPickupCubes`))
  (bind _newpickupcubes_2 (`self.NewPickupCubes`))
  (bind _mysavegame (`self.MySaveGame`))
  (bind _pickupcubes (`/Game/Button/MySaveGame.pickupCubes` _mysavegame))
  (set `self.Is Tracking` false)
  (`SceneComponent.K2_SetWorldLocation` (`self.VRButton`) (`self.Button Initial Location`) false false)
  (switch `/Game/Button/VRPushButtonEnum` (`self.Function`)
    (:`NewEnumerator0`
      ;[1 1 1] Reset: load empty savegame
      (bind _returnvalue_2 (`GameplayStatics.CreateSaveGameObject` "/Game/Button/MySaveGame.MySaveGame_C"))
      (set `self.MySaveGame` _returnvalue_2)
      ;[1 1 1] add shutter
      (`KismetArrayLibrary.Array_Add` (`/Game/Button/MySaveGame.pickupCubes` (`self.MySaveGame`)) (make `/Game/Button/StructSavePickupCube` "schuifraam" -1 "zuurkast_rail" "rail.in" (`KismetMathLibrary.MakeTransform` (0.0 0.0 80.0))) :!label _label)
      (bind _outactors (`GameplayStatics.GetAllActorsOfClass` "/Game/VirtualRealityBP/Blueprints/BP_PickupCube.BP_PickupCube_C" :!label _label_2))
      (`KismetArrayLibrary.Array_Clear` _newpickupcubes_2)
      (for (_array_element _array_index) _pickupcubes
        (bind (_staticmesh _parent _parentsocket _attachedsocket _transform _tubeend _subtype) (break `/Game/Button/StructSavePickupCube` _array_element))
        (switch `/Game/Button/MySaveObjecyType` _subtype
          (:`NewEnumerator0`
            (bind _returnvalue_3 (`|SpawnActorFromClass` "/Game/VirtualRealityBP/Blueprints/BP_PickupCube.BP_PickupCube_C" _returnvalue "Undefined" "OverrideRootScale" null null :!label _label_3))
            (`KismetArrayLibrary.Array_Add` (`self.NewPickupCubes`) _returnvalue_3))
          (:`NewEnumerator1`
            (bind _returnvalue_4 (`|SpawnActorFromClass` "/Game/glassware/TubeEnd.TubeEnd_C" _returnvalue "Undefined" "OverrideRootScale" null null))
            (`KismetArrayLibrary.Array_Add` (`self.NewPickupCubes`) _returnvalue_4))
          (:`NewEnumerator2`
            (for _array_element_2 _outactors
              (if (`/Game/VirtualRealityBP/Blueprints/BP_PickupCube._stockItem` _array_element_2)
                (if (`KismetStringLibrary.EqualEqual_StrStr` (`KismetSystemLibrary.GetObjectName` _array_element_2) _staticmesh)
                  (`|ExecutionSequence`
                    (:`then_0`
                      (bind _returnvalue_5 (`|SpawnActorFromClass` (`GameplayStatics.GetObjectClass` _array_element_2) _returnvalue "Undefined" "OverrideRootScale" null null))
                      (`KismetArrayLibrary.Array_Add` (`self.NewPickupCubes`) _returnvalue_5))
                    (:`then_1`
                      (break)))))))
          (:`NewEnumerator3`
            (for _array_element_3 _outactors
              (if (`KismetStringLibrary.EqualEqual_StrStr` (`KismetSystemLibrary.GetObjectName` _array_element_3) _staticmesh)
                (`KismetArrayLibrary.Array_Add` (`self.NewPickupCubes`) _array_element_3)
                (break)))
            (if (<= (`KismetArrayLibrary.Array_Length` (`self.NewPickupCubes`)) _array_index)
              (`KismetSystemLibrary.PrintString` (`KismetStringLibrary.Concat_StrStr` _staticmesh " not found"))
              (goto _label_3)))))
      (`/Game/Button/MySaveGame.loadSaveGame` _mysavegame _outactors _newpickupcubes_2)
      ;[1 1 1] cleanout old tubes
      (bind _outactors_2 (`GameplayStatics.GetAllActorsOfClass` "/Game/glassware/Tube1.Tube1_C"))
      (for _array_element_4 _outactors_2
        (if (not (`/Game/glassware/Tube1._stockItem` _array_element_4))
          (`self.K2_DestroyActor` _array_element_4)))
      ;[1 1 1] spawn new tubes
      (for (_array_element_5 _array_index_2) _pickupcubes
        (bind (_staticmesh_2 _parent_2 _parentsocket_2 _attachedsocket_2 _transform_2 _tubeend_2) (break `/Game/Button/StructSavePickupCube` _array_element_5))
        (if (>= _tubeend_2 0)
          (bind _astube_end (cast `/Game/glassware/TubeEnd` (`|GetArrayItem` _newpickupcubes _array_index_2)))
          (bind _astube_end_2 (cast `/Game/glassware/TubeEnd` (`|GetArrayItem` _newpickupcubes _tubeend_2)))
          (bind _returnvalue_6 (`|SpawnActorFromClass` "/Game/glassware/Tube1.Tube1_C" _transform_2 "Undefined" "OverrideRootScale" null null))
          (`self.K2_DestroyActor` (`/Game/glassware/Tube1.TubeStart` _returnvalue_6))
          (set `/Game/glassware/Tube1.TubeStart` _astube_end _returnvalue_6)
          (`self.SetOwner` _astube_end _returnvalue_6)
          (`self.K2_DestroyActor` (`/Game/glassware/Tube1.TubeEnd` _returnvalue_6))
          (set `/Game/glassware/Tube1.TubeEnd` _astube_end_2 _returnvalue_6)
          (`self.SetOwner` _astube_end_2 _returnvalue_6)
          (set `/Game/glassware/Tube1._stockItem` false _returnvalue_6)))
      ;[1 1 1] reset permanent objects
      (for _array_element_6 _outactors
        (`/Engine/EditorBlueprintResources/StandardMacros.IsValid` _array_element_6
          (:`Is Valid`
            (if (not (`/Game/VirtualRealityBP/Blueprints/BP_PickupCube._stockItem` _array_element_6))
              (bind _staticmeshcomponent (`StaticMeshActor.StaticMeshComponent` _array_element_6))
              (`/Engine/EditorBlueprintResources/StandardMacros.IsValid` (`ActorComponent.GetOwner` _staticmeshcomponent)
                (:`Is Not Valid`
                  (if (`|EnumEquality` (`SceneComponent.Mobility` _staticmeshcomponent) "Movable")
                    (`SceneComponent.K2_SetRelativeTransform` _staticmeshcomponent (`KismetMathLibrary.MakeTransform` (0.0 0.0 0.0)) false false)))))))))
    (:`NewEnumerator1`
      (bind _returnvalue_7 (`GameplayStatics.CreateSaveGameObject` "/Game/Button/MySaveGame.MySaveGame_C"))
      (bind _outactors_3 (`GameplayStatics.GetAllActorsOfClass` "/Game/VirtualRealityBP/Blueprints/BP_PickupCube.BP_PickupCube_C"))
      (`/Game/Button/MySaveGame.saveSaveGame` _returnvalue_7 _outactors_3))
    (:`NewEnumerator2`
      (bind _returnvalue_8 (`GameplayStatics.DoesSaveGameExist` "DefaultSlot" :!label _label_4))
      (if _returnvalue_8
        (bind _returnvalue_9 (`GameplayStatics.LoadGameFromSlot` "DefaultSlot"))
        (bind _asmy_save_game (cast `/Game/Button/MySaveGame` _returnvalue_9)
          (:`then`
            (set `self.MySaveGame` _asmy_save_game))
          (:`CastFailed`
            (bind _returnvalue_10 (`GameplayStatics.CreateSaveGameObject` "/Game/Button/MySaveGame.MySaveGame_C" :!label _label_5))
            (set `self.MySaveGame` _returnvalue_10)))
        (else
          (goto _label_5)))
      ;[1 1 1] Schuifraam in savegame?
      (for (_array_element_7 _array_index_3) (`/Game/Button/MySaveGame.pickupCubes` (`self.MySaveGame`))
        (if (`KismetStringLibrary.EqualEqual_StrStr` (`.StaticMesh_2_8CB49EFF40EA7E380D0292AD7A1C9A74` (break `/Game/Button/StructSavePickupCube` _array_element_7)) "schuifraam")
          (set `self.schuifraam_index` _array_index_3)
          (break)))
      (if (>= (`self.schuifraam_index`) 0)
        (goto _label_2)
        (else
          (goto _label))))))

(event `self.ReceiveBeginPlay`
  (set `self.Button Initial Location` (`SceneComponent.K2_GetComponentLocation` (`self.VRButton`)))
  (switch `/Game/Button/VRPushButtonEnum` (`self.Function`)
    (:`NewEnumerator2`
      (`|ExecutionSequence`
        (:`then_0`
          (goto _label_4))))))

(fn `UserConstructionScript`)